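; Base enemy AI character that patrols, detects and fights the player, taking damage with random stuns until death.
; SetAIState mirrors state to the controller's Blackboard and drives walk speed, HP bar and caution sign.
; Attacks pick random montages by distance and special chance, with helpers for cooldowns, projectiles and turning or moving to the player.
; Timed traces trigger obstacle jumps when engaged and hide the blocked caution sign; patrol points ping-pong.
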(event Custom|TakeDamage
  (params (InDamage :type Float%20%28double-precision%29))
  (if (not (Variables|Default|GetbIsDead?))
    (bind _output_get (Variables|Default|SetHealth (Math|Float|Clamp(Float) (- (Variables|Default|GetHealth) InDamage) 0.0 (- (Variables|Default|GetHealth) InDamage))))
    (if (<= _output_get 0.0)
      (CallFunction|PerformDeath))))

(event Custom|Dead
  ;[0.06771 0.06771 0.06771] Dead
  (if (Utilities|Enum|NotEqual(Enum) (Variables|AI|GetAIState) "NewEnumerator4")
    (CallFunction|SetAIState "NewEnumerator4")
    (AI|Components|Blackboard|SetValueasEnum (AI|GetBlackboard (Variables|Default|GetGDTVAIController)) (Utilities|Name|MakeLiteralName "AIState") (Utilities|Enum|LiteralenumS_AIState "NewEnumerator4"))
    ;;[1 1 1] Don't forget to loop montage
    (Animation|PlayAnimMontage (CallFunction|SelectDeathMontage) 1.0 "None")
    (Actor|SetLifeSpan 5.0)))

(event Custom|MoveToTarget
  (params (Speed :type Float%20%28single-precision%29))
  ;[1 1 1] rotate to target
  (Timeline|Timeline_0 PlayFromStart
    (:Update
      (Transformation|SetActorLocation (Math|Interpolation|VInterpTo (Transformation|GetActorLocation) (Transformation|GetActorLocation (Game|GetPlayerCharacter 0)) (Utilities|Time|GetWorldDeltaSeconds) Speed) false false))))

(event Custom|StopMoveToTarget
  ;[1 1 1] rotate to target
  (Timeline|Timeline_0 Stop
    (:Update
      (Transformation|SetActorLocation (Math|Interpolation|VInterpTo (Transformation|GetActorLocation) (Transformation|GetActorLocation (Game|GetPlayerCharacter 0)) (Utilities|Time|GetWorldDeltaSeconds) (stale Custom|MoveToTarget Speed)) false false))))

(event Custom|ShowCautiousSign
  (bind _cautioussign (Variables|Default|GetCautiousSign))
  ;[1 1 1] Don't show sign if vision is blocked
  (if (Utilities|Enum|Equal(Enum) (Variables|AI|GetAIState) "NewEnumerator1")
    (bind _returnvalue (Collision|LineTraceByChannel (Transformation|GetWorldLocation (Variables|Default|GetCautiousSign)) (Transformation|GetWorldLocation (Actor|GetComponentbyClass (Game|GetPlayerCharacter 0) "/Script/Engine.CameraComponent")) "TraceTypeQuery1" false 0 "ForDuration"))
    (if _returnvalue
      (Development|SetHiddeninGame _cautioussign true false)
      (else
        (Development|SetHiddeninGame _cautioussign false false)))))

(event Custom|PerformDeath
  (Variables|Default|SetbIsDead? true)
  (Animation|Montage|PlayMontage (Variables|Character|GetMesh) (.OutItem (Utilities|Array|Random (Variables|AI|Animations|Death|GetDeathMontage)))
    (:then
      (CallFunction|SetAIState "NewEnumerator4")
      (Actor|SetLifeSpan 8.0))))

(event Custom|RotateToTarget
  (params (RotateSpeed :type Float%20%28single-precision%29))
  (bind _returnvalue (Transformation|GetActorRotation))
  (bind (_roll _pitch) (Math|Rotator|BreakRotator _returnvalue))
  ;[1 1 1] rotate to target
  (Timeline|Timeline PlayFromStart
    (:Update
      (Transformation|SetActorRotation (Math|Rotator|MakeRotator _roll _pitch (.yaw (Math|Interpolation|RInterpTo _returnvalue (Math|Rotator|FindLookatRotation (Transformation|GetActorLocation) (Transformation|GetActorLocation (Game|GetPlayerCharacter 0))) (Utilities|Time|GetWorldDeltaSeconds) RotateSpeed)))))))

(event Custom|StopRotatingToTarget
  (bind _returnvalue (Transformation|GetActorRotation))
  (bind (_roll _pitch) (Math|Rotator|BreakRotator _returnvalue))
  ;[1 1 1] rotate to target
  (Timeline|Timeline Stop
    (:Update
      (Transformation|SetActorRotation (Math|Rotator|MakeRotator _roll _pitch (.yaw (Math|Interpolation|RInterpTo _returnvalue (Math|Rotator|FindLookatRotation (Transformation|GetActorLocation) (Transformation|GetActorLocation (Game|GetPlayerCharacter 0))) (Utilities|Time|GetWorldDeltaSeconds) (stale Custom|RotateToTarget RotateSpeed))))))))

(event Custom|CooldownAttack
  (Utilities|Time|SetTimerbyEvent (delegate Custom|FinishedCooldown) (Math|Random|RandomFloatinRange (Variables|AI|Attack|GetAttackCoolDownMin) (Variables|AI|Attack|GetAttackCoolDownMax))))

(event Custom|FinishedCooldown
  (CallFunction|SetCooldownKey false))

(event Custom|Attack
  ;[1 0 0] Attack
  (Animation|Montage|PlayMontage (Variables|Character|GetMesh) (CallFunction|SelectAttackMontage)
    (:OnCompleted
      _)
    (:OnBlendOut
      _)
    (:OnInterrupted
      _)
    (:OnNotifyEnd
      _))
  (CallFunction|SetAIState "NewEnumerator2"))

(event Custom|FixAttackLoopBug
  (CallFunction|SetAIState "NewEnumerator2"))

(event EventBeginPlay
  (bind _charactermovement (Variables|Character|GetCharacterMovement))
  (bind _aistate (Variables|AI|GetAIState))
  (Default|Init (.AsWBP%20HPBar (Utilities|Casting|CastToWBP_HPBar (UserInterface|GetUserWidgetObject (Variables|Default|GetHPBar)))) self)
  (Variables|/Script/Engine.CharacterMovementComponent|SetJumpZVelocity _charactermovement (Variables|AI|Movement|GetJump%20Z%20Velocity))
  (Variables|/Script/Engine.CharacterMovementComponent|SetRotationRate _charactermovement (Math|Rotator|MakeRotator 0.0 0.0 (Variables|AI|Movement|GetRotation%20Rate)))
  (Variables|Default|GetGDTVAIController
    (:then
      _)
    (:else
      (bind _asaic_base_controller (Utilities|Casting|CastToAIC_BaseController (Pawn|GetController)))
      (Variables|Default|SetGDTVAIController _asaic_base_controller)))
  (Default|Init (Variables|Default|GetGDTVAIController) (Variables|AI|GetBTAsset) (Variables|AI|Sight|GetSight%20Radius) (Variables|AI|Sight|GetLose%20Sight%20Radius) (Variables|AI|Sight|GetInstant%20Detect%20Distance) (Variables|AI|Sight|GetTime%20to%20See%20Player))
  (CallFunction|SetAIState _aistate)
  (AI|Components|Blackboard|SetValueasEnum (AI|GetBlackboard (Variables|Default|GetGDTVAIController)) (Utilities|Name|MakeLiteralName "AIState") _aistate)
  (Default|InitEgaged (Variables|Default|GetGDTVAIController))
  (Utilities|Time|SetTimerbyFunctionName 0 "JumpAndMovementCheck" 0.3 true)
  (Utilities|Time|SetTimerbyEvent (delegate Custom|ShowCautiousSign) 0.5 true)
  (EventDispatchers|BindEventtoAttackFinished (EventDispatchers|CreateEvent :!event Custom|CooldownAttack)))

(event Game|Damage|EventPointDamage
  (params (Damage :type Float%20%28single-precision%29) (DamageType :type Damage%20Type%20Object%20Reference) (HitLocation :type Vector :default "0, 0, 0") (HitNormal :type Vector :default "0, 0, 0") (HitComponent :type Primitive%20Component%20Object%20Reference) (BoneName :type Name :default "None") (ShotFromDirection :type Vector :default "0, 0, 0") (InstigatedBy :type Controller%20Object%20Reference) (DamageCauser :type Actor%20Object%20Reference) (HitInfo :type Hit%20Result%20Structure%20%28by%20ref%29))
  (CallFunction|TakeDamage Damage)
  (if (Variables|Default|GetbIsDead?)
    _
    (else
      ;[1 1 1] stun chance
      (if (< (Math|Random|RandomFloat) (Variables|Default|GetStunChance))
        (Animation|PlayAnimMontage (.OutItem (Utilities|Array|Random (Variables|AI|Animations|GetHitMontage))) 1.0 "None"))))
  (Audio|PlaySoundatLocation "/Engine/EditorSounds/GamePreview/EndSimulate_Cue.EndSimulate_Cue" HitLocation "0, 0, 0" 1.0 1.0 0.0 0 0 0 0)
  (Effects|SpawnEmitteratLocation "/Game/ParticleSystems/P_Par.P_Par" HitLocation))

(event EventTick
  (params (DeltaSeconds :type Float%20%28single-precision%29))
  (bind _hpbar (Variables|Default|GetHPBar))
  (if (Rendering|IsVisible _hpbar)
    (Transformation|SetWorldRotation _hpbar (Math|Rotator|FindLookatRotation (Transformation|GetActorLocation) (Transformation|GetWorldLocation (Actor|GetComponentbyClass (Game|GetPlayerCharacter 0) "/Script/Engine.CameraComponent"))) false false)))

(fn ConstructionScript)

(fn FindNextPatrollPoint
  (LocalVariables|SetNextPatrollPoint (Transformation|GetActorLocation (Utilities|Array|Get(acopy) (Variables|AI|Patrol|GetPatrolPoints) (Variables|AI|Patrol|GetPatrolPointCounter))))
  (if (not (Variables|AI|Patrol|GetisReversePatrol))
    ;[1 1 1] Not reverse
    (if (not (>= (+ (Variables|AI|Patrol|GetPatrolPointCounter) 1) (Utilities|Array|Length (Variables|AI|Patrol|GetPatrolPoints))))
      (Math|Integer|IncrementInt (Variables|AI|Patrol|GetPatrolPointCounter)
        (:%20%20
          _))
      (else
        (Variables|AI|Patrol|SetisReversePatrol true)
        (Math|Integer|DecrementInt (Variables|AI|Patrol|GetPatrolPointCounter)
          (:%20%20
            _))))
    (return (LocalVariables|GetNextPatrollPoint))
    (else
      ;[1 1 1] Reverse
      (if (<= (Variables|AI|Patrol|GetPatrolPointCounter) 0)
        (Variables|AI|Patrol|SetisReversePatrol false)
        (Math|Integer|IncrementInt (Variables|AI|Patrol|GetPatrolPointCounter)
          (:%20%20
            _))
        (else
          (Math|Integer|DecrementInt (Variables|AI|Patrol|GetPatrolPointCounter)
            (:%20%20
              _))))
      (return (LocalVariables|GetNextPatrollPoint)))))

(fn SetAIState
  (params (NewState :type S_AIState%20Enum :default "NewEnumerator5"))
  (bind _returnvalue (Utilities|Name|MakeLiteralName "AIState"))
  (bind _charactermovement (Variables|Character|GetCharacterMovement))
  (bind _gdtvaicontroller (Variables|Default|GetGDTVAIController))
  (bind _returnvalue_2 (AI|GetBlackboard _gdtvaicontroller))
  (if (Utilities|Enum|Equal(Enum) NewState (Variables|AI|GetAIState))
    (return)
    (else
      (Utilities|Time|ClearandInvalidateTimerbyHandle (Variables|Default|GetAttackLoopBugTimer))
      (Variables|Default|GetGDTVAIController
        (:then
          (switch Utilities|FlowControl|Switch|SwitchonS_AIState NewState
            (:NewEnumerator5
              (AI|Components|Blackboard|SetValueasEnum _returnvalue_2 _returnvalue (Utilities|Enum|LiteralenumS_AIState "NewEnumerator5"))
              (Variables|AI|SetAIState "NewEnumerator5")
              (Development|SetHiddeninGame (Variables|Default|GetCautiousSign) true false :!label _label)
              (Variables|/Script/Engine.CharacterMovementComponent|SetMaxWalkSpeed _charactermovement 0.0))
            (:NewEnumerator0
              (AI|Components|Blackboard|SetValueasEnum _returnvalue_2 _returnvalue (Utilities|Enum|LiteralenumS_AIState "NewEnumerator0"))
              (Variables|AI|SetAIState "NewEnumerator0")
              (Development|SetHiddeninGame (Variables|Default|GetCautiousSign) true false)
              (Variables|/Script/Engine.CharacterMovementComponent|SetMaxWalkSpeed _charactermovement (Variables|AI|Movement|GetWalkSpeed) :!label _label_2))
            (:NewEnumerator1
              (AI|Components|Blackboard|SetValueasEnum _returnvalue_2 _returnvalue (Utilities|Enum|LiteralenumS_AIState "NewEnumerator1"))
              (Variables|AI|SetAIState "NewEnumerator1")
              (Development|SetHiddeninGame (Variables|Default|GetCautiousSign) false false)
              (goto _label_2))
            (:NewEnumerator2
              (AI|Components|Blackboard|SetValueasEnum _returnvalue_2 _returnvalue (Utilities|Enum|LiteralenumS_AIState "NewEnumerator2"))
              (Variables|AI|SetAIState "NewEnumerator2")
              (Development|SetHiddeninGame (Variables|Default|GetCautiousSign) true false)
              (Variables|/Script/Engine.CharacterMovementComponent|SetMaxWalkSpeed _charactermovement (Variables|AI|Movement|GetEngagedWalkSpeed)))
            (:NewEnumerator3
              (AI|Components|Blackboard|SetValueasEnum _returnvalue_2 _returnvalue (Utilities|Enum|LiteralenumS_AIState "NewEnumerator3"))
              (Variables|AI|SetAIState "NewEnumerator3")
              (goto _label))
            (:NewEnumerator6
              (AI|Components|Blackboard|SetValueasEnum _returnvalue_2 _returnvalue (Utilities|Enum|LiteralenumS_AIState "NewEnumerator6"))
              (Variables|AI|SetAIState "NewEnumerator6")
              (goto _label))
            (:NewEnumerator4
              (AI|Components|Blackboard|SetValueasEnum _returnvalue_2 _returnvalue (Utilities|Enum|LiteralenumS_AIState "NewEnumerator4"))
              (Variables|AI|SetAIState "NewEnumerator4")
              (goto _label)))
          (Rendering|SetVisibility (Variables|Default|GetHPBar) (Utilities|Enum|Equal(Enum) (Variables|AI|GetAIState) "NewEnumerator2") false)
          (return))
        (:else
          (return))))))

(fn JumpandMovementCheck
  (bind _capsulecomponent (Variables|Default|GetCapsuleComponent))
  (bind _returnvalue (Transformation|GetWorldTransform _capsulecomponent))
  (Utilities|FlowControl|Sequence
    (:then_0
      (bind _outhit (Collision|LineTraceByChannel (Math|Transform|TransformLocation _returnvalue "10.000000,0.000000,-30.000000") (Math|Transform|TransformLocation _returnvalue (Math|Vector|MakeVector (+ (/ (Math|Vector|VectorLengthXY (Variables|/Script/Engine.MovementComponent|GetVelocity (Variables|Character|GetCharacterMovement))) 4.0) (Variables|AI|Movement|GetTraceJumpDitance)) 0.0 -3e+01)) "TraceTypeQuery1" false (Utilities|Array|MakeArray (Game|GetPlayerCharacter 0)) (Variables|AI|Movement|GetTraceJumpDebug)))
      (if (Math|Boolean|ANDBoolean (Utilities|Enum|Equal(Enum) (Variables|AI|GetAIState) "NewEnumerator2") (> (Math|Vector|VectorLength (Variables|/Script/Engine.MovementComponent|GetVelocity (Variables|Character|GetCharacterMovement))) 2e+01) (.bBlockingHit (Collision|BreakHitResult _outhit)) (Math|Float|InRange(Float) (.Z (Class|KismetMathLibrary|BreakVector3f (.ImpactNormal (Collision|BreakHitResult _outhit)))) -0.1 0.1))
        (Character|Jump)))))

(fn GetSeePlayerTimeElapsed
  (bind _returnvalue (Default|GetSeePlayerTimeElapsed (Variables|Default|GetGDTVAIController)))
  (return _returnvalue))

(fn SelectAttackMontage
  (bind _returnvalue (Game|GetPlayerCharacter 0))
  (bind _returnvalue_2 (Transformation|GetActorLocation))
  (bind _specialattackmontage (Variables|AI|Attack|GetSpecialAttackMontage))
  (bind _closecombatradius (Variables|AI|Combat|GetCloseCombatRadius))
  (bind _rangespecialattackmontage (Variables|AI|Attack|GetRangeSpecialAttackMontage))
  (bind _outitem (Utilities|Array|Random _rangespecialattackmontage))
  (bind _outitem_2 (Utilities|Array|Random _specialattackmontage))
  (bind _returnvalue_3 (Transformation|GetActorLocation _returnvalue))
  (bind _returnvalue_4 (Math|Vector|Distance(Vector) _returnvalue_2 _returnvalue_3))
  (bind _returnvalue_5 (<= _returnvalue_4 _closecombatradius))
  (bind _returnvalue_6 (select _returnvalue_5 _outitem_2 _outitem))
  (if (< (Math|Random|RandomFloat) (Variables|AI|Attack|GetSpecialAttackChance))
    (Utilities|IsValid _returnvalue_6
      (:Is%20Valid
        (return _returnvalue_6))
      (:Is%20Not%20Valid
        _)))
  (return (select (<= (Math|Vector|Distance(Vector) (Transformation|GetActorLocation) (Transformation|GetActorLocation (Game|GetPlayerCharacter 0))) (Variables|AI|Combat|GetCloseCombatRadius)) (.OutItem (Utilities|Array|Random (Variables|AI|Attack|GetAttackMontage))) (.OutItem (Utilities|Array|Random (Variables|AI|Attack|GetRangeAttackMontage))))))

(fn SelectDeathMontage
  (return (.OutItem (Utilities|Array|Random (Variables|AI|Animations|Death|GetDeathMontage)))))

(fn SpawnProjectile
  (params (SocketName :type Name) (ProjectileClass :type BP%20Base%20Projectile%20Class%20Reference))
  (bind _self self)
  (bind _returnvalue (Game|SpawnActorfromClass ProjectileClass (Math|Transform|MakeTransform (Transformation|GetSocketLocation (Variables|Character|GetMesh) SocketName) "0, 0, 0" "1.000000,1.000000,1.000000") "Undefined" _self 0 _self))
  (Variables|/Script/Engine.MovementComponent|SetVelocity (Variables|/Game/AI/Projectile/BP_BaseProjectile.BP_BaseProjectile_C|GetProjectileMovement _returnvalue) (* (Math|Vector|Normalize (- (Transformation|GetActorLocation (Game|GetPlayerCharacter 0)) (Transformation|GetActorLocation))) (Class|MovementComponent|GetMaxSpeed (Variables|/Game/AI/Projectile/BP_BaseProjectile.BP_BaseProjectile_C|GetProjectileMovement _returnvalue))))
  (return))

(fn SetCooldownKey
  (params (BoolValue :type Boolean))
  (AI|Components|Blackboard|SetValueasBool (AI|GetBlackboard (Variables|Default|GetGDTVAIController)) (Utilities|Name|MakeLiteralName "IsAttackCooldown") BoolValue)
  (return))

(fn AIApplyDamage
  (params (Hit :type Hit%20Result%20Structure%20%28by%20ref%29) (BaseDamage :type Float%20%28single-precision%29))
  (Game|Damage|ApplyPointDamage (.HitActor (Collision|BreakHitResult Hit)) BaseDamage (Transformation|GetActorForwardVector (Components|GetOwner)) Hit (Game|GetInstigatorController) self))