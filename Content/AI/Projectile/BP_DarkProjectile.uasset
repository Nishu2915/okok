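; BP_DarkProjectile is an AI projectile actor that shows a Niagara effect in flight and expires after a fixed lifespan.
; The first blocking bounce reported by ProjectileMovement serves as the impact, spawning one Niagara effect for Character hits and another for anything else, then destroying the projectile.
; Impact effects are oriented to the surface normal using the projectile's rotated forward vector.
; The graph applies no damage.
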(event OnProjectileBounce(ProjectileMovement)
  (params (ImpactResult :type Hit%20Result%20Structure%20%28by%20ref%29) (ImpactVelocity :type Vector%20%28by%20ref%29 :default "0, 0, 0"))
  (bind (_bblockinghit _binitialoverlap _time _distance _location _impactpoint _normal _impactnormal _physmat _hitactor) (Collision|BreakHitResult ImpactResult))
  (bind _returnvalue (Transformation|GetActorUpVector))
  (bind _returnvalue_2 (Transformation|GetActorForwardVector))
  (bind _returnvalue_3 (Math|Vector|DotProduct _normal _returnvalue))
  (bind _returnvalue_4 (Math|Vector|CrossProduct _normal _returnvalue))
  (bind _returnvalue_5 (Class|KismetMathLibrary|DegAcos _returnvalue_3))
  (bind _returnvalue_6 (Math|Vector|Normalize _returnvalue_4))
  (bind _returnvalue_7 (Math|Vector|RotateVectorAroundAxis _returnvalue_2 _returnvalue_5 _returnvalue_6))
  (bind _returnvalue_8 (Math|Rotator|MakeRotfromZX _normal _returnvalue_7))
  (if _bblockinghit
    (if (.bSuccess (Utilities|Casting|CastToCharacter _hitactor))
      (Niagara|SpawnSystematLocation (Variables|Default|GetHitActorEffect) _impactpoint _returnvalue_8)
      (else
        (Niagara|SpawnSystematLocation (Variables|Default|GetHitNonActorEffect) _impactpoint _returnvalue_8)))
    (Actor|DestroyActor)))

(event EventBeginPlay
  (Class|NiagaraComponent|SetAsset (Variables|Default|GetNiagara) (Variables|Default|GetAttachedEffect) true)
  (Actor|SetLifeSpan 1e+01))

(fn ConstructionScript)