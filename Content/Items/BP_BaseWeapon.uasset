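; Base weapon item that attaches to its owner on equip and deals point damage on hit.
; Equipping registers it as the combat component's main weapon, picks the hand or attach socket by combat state, and sends its combat type to the owner's AnimInstance.
; The collision component traces the item mesh, ignoring the owner, and its OnHit event applies the damage.
; A separate event switches the mesh to physics simulation.
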(event OnHit(BPC_CollisionComponent)
  (params (HitResult :type Hit%20Result%20Structure))
  (Game|Damage|ApplyPointDamage (.HitActor (Collision|BreakHitResult HitResult)) (Variables|Default|GetDamage) (Transformation|GetActorForwardVector (Components|GetOwner)) HitResult (Game|GetInstigatorController) self))

(event Custom|SimulateWeaponPhysic
  (bind _returnvalue (CallFunction|GetItemMesh))
  (Collision|SetCollisionProfileName _returnvalue "PhysicsActor" true :!class /Script/Engine.PrimitiveComponent)
  (Physics|SetSimulatePhysics _returnvalue true))

(event EventBeginPlay
  (|CallParentFunction) ; This node is disabled and will not be called.\nDrag off pins to build functionality.
)

(event Collision|EventActorBeginOverlap
  (params (OtherActor :type Actor%20Object%20Reference))
  (|CallParentFunction OtherActor) ; This node is disabled and will not be called.\nDrag off pins to build functionality.
)

(event EventTick
  (params (DeltaSeconds :type Float%20%28single-precision%29))
  (|CallParentFunction DeltaSeconds) ; This node is disabled and will not be called.\nDrag off pins to build functionality.
)

(fn ConstructionScript
  (|CallParentFunction))

(fn OnEquipped
  (bind _bpc_collisioncomponent (Variables|Default|GetBPC_CollisionComponent))
  (|CallParentFunction)
  (Variables|Default|GetCombatComponent
    (:then
      _)
    (:else
      (Variables|Default|SetCombatComponent (Actor|GetComponentbyClass (Components|GetOwner) "/Game/Components/BPC_CombatComponent.BPC_CombatComponent_C"))))
  (CallFunction|SetIsEquipped true)
  (CallFunction|AttachActor (select (Default|IsCombatEnabled? (Variables|Default|GetCombatComponent)) (Variables|Initialization|GetHandSocketName) (Variables|Default|GetAttachSocketName)))
  (Default|SetMainWeapon (Variables|Default|GetCombatComponent) self)
  (Class|BPIAnimInstance|UpdateCombatType(Message) (Components|SkeletalMesh|GetAnimInstance (Variables|/Script/Engine.Character|GetMesh (.AsCharacter (Utilities|Casting|CastToCharacter (Components|GetOwner))))) (Variables|Initialization|GetCombatType))
  (Default|SetCollisionMesh _bpc_collisioncomponent (CallFunction|GetItemMesh))
  (Default|AddActortoIgnore _bpc_collisioncomponent (Components|GetOwner)))