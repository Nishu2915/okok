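; Player character Blueprint that handles walk and sprint movement, with placeholder attack and block input events.
; Pressing sprint while moving switches the speed mode, which sets CharacterMovement max walk speed, and starts a looping SprintStaminaCost timer, though that function is not defined here.
; Releasing sprint clears the timer and restores walking.
; Attack and block only check whether something is equipped and take no action yet.
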(event Custom|DisableSprint
  ;[0.00089 1 0] Walk/Sprint
  (Utilities|Time|ClearTimerbyFunctionName 0 "SprintStaminaCost")
  (if (Utilities|Enum|Equal(Enum) (CallFunction|GetCurrentSpeedMode) "Sprint")
    (CallFunction|SetMovementSpeedMode "Walk")))

(event EventBeginPlay
  ;[1 1 1] BeginPlay
)

(event EventOnAttackPressed
  (params (Value :type Input%20Action%20Value%20Structure%20%28by%20ref%29))
  (if (Class|GDTVPlayerCharacter|IsEquipped)
    _))

(event EventOnBlockPressed
  (params (Value :type Input%20Action%20Value%20Structure%20%28by%20ref%29))
  (if (Class|GDTVPlayerCharacter|IsEquipped)
    _))

(event EventOnSprintPressed
  (params (Value :type Input%20Action%20Value%20Structure%20%28by%20ref%29))
  ;[0.00089 1 0] Walk/Sprint
  (if (CallFunction|CanPerformSprint)
    (CallFunction|SetMovementSpeedMode "Sprint")
    (Utilities|Time|SetTimerbyFunctionName 0 "SprintStaminaCost" 0.1 true)))

(event EventOnSprintReleased
  (params (Value :type Input%20Action%20Value%20Structure%20%28by%20ref%29))
  ;[0.00089 1 0] Walk/Sprint
  (CallFunction|DisableSprint))

(event EventSetMovementMode
  (params (Mode :type EMovementSpeedMode%20Enum :default "Crouch"))
  ;[0.00089 1 0] Walk/Sprint
  (CallFunction|SetMovementSpeedMode Mode))

(fn ConstructionScript)

(fn SetMovementSpeedMode
  (params (MovementSpeedMode :type EMovementSpeedMode%20Enum :default "Crouch"))
  (bind _charactermovement (Variables|Character|GetCharacterMovement))
  (if (Utilities|Enum|NotEqual(Enum) MovementSpeedMode (Variables|Default|GetMovementSpeedMode))
    (bind _output_get (Variables|Default|SetMovementSpeedMode MovementSpeedMode))
    (switch Utilities|FlowControl|Switch|SwitchonEMovementSpeedMode _output_get
      (:Walk
        (Variables|/Script/Engine.CharacterMovementComponent|SetMaxWalkSpeed _charactermovement (Variables|Default|GetWalkSpeed)))
      (:Sprint
        (Variables|/Script/Engine.CharacterMovementComponent|SetMaxWalkSpeed _charactermovement (Variables|Default|GetSprintSpeed))))))

(fn GetCurrentSpeedMode
  (return (Variables|Default|GetMovementSpeedMode)))

(fn CanPerformSprint
  (return (!= (Math|Vector|VectorLength (Transformation|GetVelocity)) 0.0)))